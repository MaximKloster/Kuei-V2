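; Physics object that the ghost character can push around with its hands.
; Mesh overlaps with the character's tagged left or right hand collision flag that hand as active and record its position.
; Each tick, the active hand's movement since the last frame becomes a force on the mesh, scaled by GhostPower and Mass, with the right hand taking priority.
; The construction script derives the mesh's mass scale from Mass.
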(event OnComponentBeginOverlap(Mesh)
  (params (OtherActor :type Actor%20Object%20Reference) (OtherComp :type Primitive%20Component%20Object%20Reference) (OtherBodyIndex :type Integer) (bFromSweep :type Boolean) (SweepResult :type Hit%20Result%20Structure%20%28by%20ref%29))
  (bind _returnvalue (Transformation|GetWorldLocation OtherComp))
  ;[1 1 1] Check and set active hand changing for this object
  (bind _asbp_ghost_charakter (Utilities|Casting|CastToBP_GhostCharakter OtherActor))
  (Variables|Default|SetCharakter _asbp_ghost_charakter)
  (if (Components|ComponentHasTag OtherComp "RightHandCollision")
    (Variables|Default|SetRightHandInAction true)
    (Variables|Default|SetRightHandTouchStartPosition _returnvalue)
    (elif (Components|ComponentHasTag OtherComp "LeftHandCollision")
      (Variables|Default|SetLeftHandInAction true)
      (Variables|Default|SetLeftHandTouchStartPosition _returnvalue))))

(event OnComponentEndOverlap(Mesh)
  (params (OtherActor :type Actor%20Object%20Reference) (OtherComp :type Primitive%20Component%20Object%20Reference) (OtherBodyIndex :type Integer))
  ;[1 1 1] Remove active hand if its not more overlaped
  (Utilities|Casting|CastToBP_GhostCharakter OtherActor)
  (if (Components|ComponentHasTag OtherComp "RightHandCollision")
    (Variables|Default|SetRightHandInAction false)
    (elif (Components|ComponentHasTag OtherComp "LeftHandCollision")
      (Variables|Default|SetLeftHandInAction false))))

(event EventTick
  (params (DeltaSeconds :type Float%20%28single-precision%29))
  (bind _charakter (Variables|Default|GetCharakter))
  (bind _charakter_2 (Variables|Default|GetCharakter))
  ;[1 1 1] Position changes by righ hand in action
  (if (Variables|Default|GetRightHandInAction)
    (bind (_newposition _force) (CallFunction|CalculateForce (Transformation|GetWorldLocation (Variables|/Game/Blueprints/BP_GhostCharakter.BP_GhostCharakter_C|GetCollisionRightHandBox _charakter)) (Variables|Default|GetRightHandTouchStartPosition) (Variables|/Game/Blueprints/BP_GhostCharakter.BP_GhostCharakter_C|GetGhostPower _charakter)))
    (Variables|Default|SetRightHandTouchStartPosition _newposition)
    (Physics|AddForce (Variables|Default|GetMesh) _force "None" false)
    (else
      ;[1 1 1] Position changes by left hand in action
      (if (Variables|Default|GetLeftHandInAction)
        (bind (_newposition_2 _force_2) (CallFunction|CalculateForce (Transformation|GetWorldLocation (Variables|/Game/Blueprints/BP_GhostCharakter.BP_GhostCharakter_C|GetCollisionLeftHandBox _charakter_2)) (Variables|Default|GetLeftHandTouchStartPosition) (Variables|/Game/Blueprints/BP_GhostCharakter.BP_GhostCharakter_C|GetGhostPower _charakter_2)))
        (Variables|Default|SetLeftHandTouchStartPosition _newposition_2)
        (Physics|AddForce (Variables|Default|GetMesh) _force_2 "None" false)))))

(fn ConstructionScript
  (Class|PrimitiveComponent|SetMassScale (Variables|Default|GetMesh) "None" (/ (Variables|Default|GetMass) 1e+03)))

(fn CalculateForce
  (params (ChangedPostion :type Vector) (StartPosition :type Vector) (GhostPower :type Float%20%28single-precision%29))
  (bind _returnvalue (- ChangedPostion StartPosition))
  (bind _returnvalue_2 (* _returnvalue 5.0))
  (return ChangedPostion (* (+ _returnvalue_2 (* (/ _returnvalue_2 (Variables|Default|GetMass)) 1e+03)) GhostPower)))