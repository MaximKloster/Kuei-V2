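; BP_SizerShower is a height marker actor that shows a given Height as a thin mesh bar with a text label in meters.
; Its construction script scales the mesh from Height, raises mesh and text to half that height above the root, and nudges the text forward.
; The label converts Height from centimeters to meters, and the event graph holds only disabled placeholder events, so there is no gameplay logic.
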(event EventBeginPlay)

(event Collision|EventActorBeginOverlap
  (params (OtherActor :type Actor%20Object%20Reference)))

(event EventTick
  (params (DeltaSeconds :type Float%20%28single-precision%29)))

(fn ConstructionScript
  (bind _height (Variables|Default|Getheight))
  (bind _defaultsceneroot (Variables|Default|GetDefaultSceneRoot))
  (bind _returnvalue (Transformation|GetWorldLocation _defaultsceneroot))
  (bind (_x _y _z) (Math|Vector|BreakVector _returnvalue))
  (Transformation|SetWorldScale3D (Variables|Default|GetStaticMesh) (Math|Vector|MakeVector 0.05 0.1 (/ _height 256.0)))
  (Transformation|SetWorldLocation (Variables|Default|GetStaticMesh) (Math|Vector|MakeVector _x _y (+ _z (/ _height 2.0))) false)
  (Transformation|AddLocalOffset (Variables|Default|GetTextRender) "10.000000,0.000000, 0" false)
  (Rendering|Components|TextRender|SetText (Variables|Default|GetTextRender) (Utilities|Text|ToText(String) (Utilities|String|Append (Utilities|String|ToString(Float) (/ _height 1e+02)) " m"))))