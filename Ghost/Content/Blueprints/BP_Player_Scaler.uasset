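; BP_Player_Scaler sizes itself to match the body of the player tracked by Kinect.
; Each tick it gets the centered body and sums head, spine and right-leg joint distances into PlayerSize, which scales the root on Y and Z only.
; It also records when tracking begins and derives the player's arm length from the right shoulder, elbow and wrist joints.
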(event EventTick
  (params (DeltaSeconds :type Float%20%28single-precision%29))
  (bind _kinectinterface (Variables|Default|GetKinectInterface))
  (bind (_centeredbody _istracked) (Class|KinectInterfaceComponent|GetCenteredBody _kinectinterface))
  (if _istracked
    (if (Variables|Default|GetPlayerIsTracked)
      _
      (else
        (Variables|Default|SetPlayerIsTracked true)
        (Variables|Default|SetTrackedStartTime (Utilities|Time|GetRealTimeSeconds))))
    (bind _output_get (Variables|Default|SetCenteredBody _centeredbody))
    ;[1 1 1] Get distances between joins for the size calculation
    (bind _returnvalue (Class|KinectInterfaceComponent|GetDistanceBetweenJoints _kinectinterface "Head" "Neck" _output_get))
    (bind _returnvalue_2 (Class|KinectInterfaceComponent|GetDistanceBetweenJoints _kinectinterface "FootRight" "SpineBase" _output_get))
    (bind _returnvalue_3 (Class|KinectInterfaceComponent|GetDistanceBetweenJoints _kinectinterface "Neck" "SpineBase" _output_get))
    (Variables|Default|SetPlayerSize (+ _returnvalue_3 _returnvalue_2 (* _returnvalue 2.0)))
    (Transformation|SetWorldScale3D (Variables|Default|Getroot) (Math|Vector|MakeVector 1.0 (/ (Variables|Default|GetPlayerSize) 2e+02) (/ (Variables|Default|GetPlayerSize) 2e+02)))
    (CallFunction|CalculateArmLength)
    (else
      (Variables|Default|SetPlayerIsTracked false))))

(fn ConstructionScript)

(fn CalculateArmLength
  (bind _returnvalue (Class|KinectInterfaceComponent|GetDistanceBetweenJoints (Variables|Default|GetKinectInterface) "WristRight" "ElbowRight" (Variables|Default|GetCenteredBody)))
  (bind _returnvalue_2 (Class|KinectInterfaceComponent|GetDistanceBetweenJoints (Variables|Default|GetKinectInterface) "ElbowRight" "ShoulderRight" (Variables|Default|GetCenteredBody)))
  (Variables|Default|SetArmLength (+ _returnvalue_2 _returnvalue)))