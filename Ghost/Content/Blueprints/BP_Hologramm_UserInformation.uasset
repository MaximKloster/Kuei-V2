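; Hologram display actor that shows tracked-user information: session time, player size and arm length.
; The construction script caches the first BP_Player_Scaler in the level and, only if one exists, sizes and positions the base, panel and text from width and height scale variables and applies the header.
; Tick rewrites the three text lines from that scaler, computing elapsed real time since tracking started or showing zero while untracked.
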(event EventBeginPlay)

(event Collision|EventActorBeginOverlap
  (params (OtherActor :type Actor%20Object%20Reference)))

(event EventTick
  (params (DeltaSeconds :type Float%20%28single-precision%29))
  (bind _playerscaleref (Variables|Default|GetPlayerScaleRef))
  (if (not (Variables|/Game/Blueprints/BP_Player_Scaler.BP_Player_Scaler_C|GetPlayerIsTracked _playerscaleref))
    (Rendering|Components|TextRender|SetText (Variables|Default|GetTextLine01) (Utilities|Text|ToText(String) "Time: 00:00:00"))
    (else
      (Rendering|Components|TextRender|SetText (Variables|Default|GetTextLine01) (Utilities|Text|ToText(String) (Utilities|String|Append "Time: " (Utilities|String|ToString(Text) (Class|KismetTextLibrary|AsTimespanTimespan (Math|Timespan|FromSeconds (- (Utilities|Time|GetRealTimeSeconds) (Variables|/Game/Blueprints/BP_Player_Scaler.BP_Player_Scaler_C|GetTrackedStartTime _playerscaleref))))))))))
  (Rendering|Components|TextRender|SetText (Variables|Default|GetTextLine02) (Utilities|Text|ToText(String) (Utilities|String|Append "Size: " (Utilities|String|ToString(Float) (Variables|/Game/Blueprints/BP_Player_Scaler.BP_Player_Scaler_C|GetPlayerSize _playerscaleref)))))
  (Rendering|Components|TextRender|SetText (Variables|Default|GetTextLine03) (Utilities|Text|ToText(String) (Utilities|String|Append "Arm Length: " (Utilities|String|ToString(Float) (Variables|/Game/Blueprints/BP_Player_Scaler.BP_Player_Scaler_C|GetArmLength _playerscaleref))))))

(fn ConstructionScript
  (bind _hologrammwidthscale (Variables|Default|GetHologrammWidthScale))
  (bind _hologrammheightscale (Variables|Default|GetHologrammHeightScale))
  (bind _returnvalue (* _hologrammheightscale 256.0))
  ;[0 0.006851 1] Find the Player Scaler Reference and setup the scale
  (bind _outactors (Actor|GetAllActorsOfClass "/Game/Blueprints/BP_Player_Scaler.BP_Player_Scaler_C"))
  (for (_array_element _array_index) _outactors
    (if (== _array_index 0)
      (Variables|Default|SetPlayerScaleRef _array_element)
      ;[1 1 1] Set the scale and position of the text
      (Transformation|SetWorldScale3D (Variables|Default|GetHologramBase) (Math|Vector|MakeVector 0.01 (+ _hologrammwidthscale 0.01) 0.01))
      (Transformation|SetWorldScale3D (Variables|Default|GetHologramm%20Area) (Math|Vector|MakeVector 0.005 _hologrammwidthscale (Variables|Default|GetHologrammHeightScale)))
      (Transformation|SetRelativeLocation (Variables|Default|GetHologramm%20Area) (Math|Vector|MakeVector 0.0 0.0 (* _hologrammheightscale 128.0)) false)
      (Transformation|SetRelativeLocation (Variables|Default|GetTextRoot) (Math|Vector|MakeVector 0.0 (- (* (Variables|Default|GetHologrammWidthScale) 128.0) 5.0) (- _returnvalue 3e+01)) false)
      (Transformation|SetRelativeLocation (Variables|Default|GetHeaderText) (Math|Vector|MakeVector 0.0 0.0 (- _returnvalue 1e+01)) false)
      (Rendering|Components|TextRender|SetText (Variables|Default|GetHeaderText) (Variables|Default|GetHeader)))))