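; BP_NotMoveableWall is a resizable wall that tells BP_GhostCharakter when it is inside the wall's collision.
; Overlap begin stores the ghost's moving direction and sets a collided flag, Tick keeps resending both through InNotMoveableWall, and overlap end sends the cleared flag.
; The construction script toggles wall visibility and, for a non-zero EndPoint, scales, centers and yaws the mesh to span from the actor to that point.
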(event OnComponentEndOverlap(Collision)
  (params (OtherActor :type Actor%20Object%20Reference) (OtherComp :type Primitive%20Component%20Object%20Reference) (OtherBodyIndex :type Integer))
  (bind _asbp_ghost_charakter (Utilities|Casting|CastToBP_GhostCharakter OtherActor))
  (bind _output_get (Variables|Default|SetCharakterCollided false))
  (Default|InNotMoveableWall _asbp_ghost_charakter _output_get (Variables|Default|GetMovingDiriction)))

(event OnComponentBeginOverlap(Collision)
  (params (OtherActor :type Actor%20Object%20Reference) (OtherComp :type Primitive%20Component%20Object%20Reference) (OtherBodyIndex :type Integer) (bFromSweep :type Boolean) (SweepResult :type Hit%20Result%20Structure%20%28by%20ref%29))
  (bind _asbp_ghost_charakter (Utilities|Casting|CastToBP_GhostCharakter OtherActor))
  (bind _output_get (Variables|Default|SetCharakter _asbp_ghost_charakter))
  (bind _output_get_2 (Variables|Default|SetMovingDiriction (Variables|/Game/Blueprints/BP_GhostCharakter.BP_GhostCharakter_C|GetMovingDiriction _output_get)))
  (bind _output_get_3 (Variables|Default|SetCharakterCollided true))
  (Default|InNotMoveableWall _asbp_ghost_charakter _output_get_3 _output_get_2))

(event EventTick
  (params (DeltaSeconds :type Float%20%28single-precision%29))
  (bind _charaktercollided (Variables|Default|GetCharakterCollided))
  (if _charaktercollided
    (Default|InNotMoveableWall (Variables|Default|GetCharakter) _charaktercollided (Variables|Default|GetMovingDiriction))))

(fn ConstructionScript
  (bind _returnvalue (Transformation|GetActorLocation))
  (bind _endpoint (Variables|Default|GetEndPoint))
  (bind _wall (Variables|Default|GetWall))
  (bind (_x _y) (Math|Vector|BreakVector _endpoint))
  (Rendering|SetVisibility _wall (Variables|Default|GetVisibil) false)
  (if (Math|Vector|NotEqual(Vector) _endpoint "0, 0, 0" 0.0001)
    ;[1 1 1] Setup the wall size
    (Transformation|SetWorldScale3D _wall (Math|Vector|MakeVector (/ (Math|Vector|VectorLength _endpoint) 256.0) (/ (Variables|Default|GetWallSickness) 256.0) (/ (Variables|Default|GetWallHight) 256.0)))
    ;[1 1 1] Setup the wall position
    (Transformation|SetRelativeLocation (Variables|Default|GetWall) (Math|Vector|MakeVector (/ _x 2.0) (/ _y 2.0) (/ (Variables|Default|GetWallHight) 2.0)) false)
    ;[1 1 1] Setup the wall rotation
    (Transformation|SetWorldRotation (Variables|Default|GetWall) (Class|KismetMathLibrary|MakeRot 0.0 (.Yaw (Class|KismetMathLibrary|BreakRot (Math|Rotator|FindLookatRotation _returnvalue (+ _returnvalue _endpoint)))) 0.0) false)))