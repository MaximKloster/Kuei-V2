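; BP_RoofLamp is a roof lamp actor with a spotlight and two tube meshes that can be switched on or off.
; The construction script applies the color, on state and intensity variables to the light, without touching the tube materials.
; SetLight toggles spotlight visibility and swaps both tubes between a lit material and a glass one.
; The event graph has no active logic, so switching relies on external calls to SetLight.
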(event EventBeginPlay)

(event Collision|EventActorBeginOverlap
  (params (OtherActor :type Actor%20Object%20Reference)))

(event EventTick
  (params (DeltaSeconds :type Float%20%28single-precision%29)))

(fn ConstructionScript
  (bind _spotlight (Variables|Default|GetSpotLight))
  (Rendering|Components|Light|SetLightColor _spotlight (Variables|LightningSettings|GetLightColor))
  (Rendering|SetVisibility _spotlight (Variables|LightningSettings|GetIsOn) false)
  (Rendering|Components|Light|SetIntensity (Variables|LightningSettings|GetIntensity)))

(fn SetLight
  (params (IsOn :type Boolean))
  (bind _tube (Variables|Default|GetTube))
  (bind _tube1 (Variables|Default|GetTube1))
  (Rendering|SetVisibility (Variables|Default|GetSpotLight) IsOn false)
  (if IsOn
    (Rendering|Material|SetMaterial _tube 0 "/Game/Materials/M_LightTube_ON.M_LightTube_ON")
    (Rendering|Material|SetMaterial _tube1 0 "/Game/Materials/M_LightTube_ON.M_LightTube_ON")
    (else
      (Rendering|Material|SetMaterial _tube 0 "/Game/Materials/MIC_Glass_Tube.MIC_Glass_Tube")
      (Rendering|Material|SetMaterial _tube1 0 "/Game/Materials/MIC_Glass_Tube.MIC_Glass_Tube"))))