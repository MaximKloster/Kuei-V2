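; Hologram message display actor that opens and closes with a sound, showing a header and wrapped message text.
; ActivateHologram starts a Tick-driven PlayHologram, which grows or shrinks the panel by a fixed per-frame step through SetHologramPosition.
; Once open, CreateTextInLines wraps the message by measuring a hidden test line, then fills up to ten text components; only the Instant style is handled.
; The construction script previews size, header and open state.
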(event EventBeginPlay)

(event Collision|EventActorBeginOverlap
  (params (OtherActor :type Actor%20Object%20Reference)))

(event EventTick
  (params (DeltaSeconds :type Float%20%28single-precision%29))
  (if (Variables|Default|GetHologramActivated)
    (CallFunction|PlayHologram)))

(fn ConstructionScript
  ;[1 1 1] Set the scale and position of the hologram
  (Rendering|SetVisibility (Variables|Default|GetTestTextLine) false false)
  (Transformation|SetWorldScale3D (Variables|Default|GetHologramBase) (Math|Vector|MakeVector 0.01 (+ (Variables|Default|GetHologramWidthScale) 0.01) 0.01))
  (if (Variables|Default|GetHologramIsOpen)
    (CallFunction|SetHologramPosition (Variables|Default|GetHologramHeightScale))
    (CallFunction|CreateTextinLines (Variables|Default|GetShown%20Text))
    (else
      (CallFunction|SetHologramPosition 0.0)))
  (Rendering|Components|TextRender|SetText (Variables|Default|GetHeaderText) (Variables|Default|GetHeader)))

(fn ActivateHologram
  (bind _defaultsceneroot (Variables|Default|GetDefaultSceneRoot))
  (bind _returnvalue (Transformation|GetWorldLocation _defaultsceneroot))
  (if (Variables|Default|GetHologramIsOpen)
    (Variables|Default|SetHologramCurrentPosition (Variables|Default|GetHologramHeightScale))
    (Audio|PlaySoundatLocation "/Game/Audio/digital_camera_switch_off_lens_in.digital_camera_switch_off_lens_in" _returnvalue)
    (else
      (Variables|Default|SetHologramCurrentPosition 0.0)
      (Audio|PlaySoundatLocation "/Game/Audio/digital_camera_switch_on_lens_out.digital_camera_switch_on_lens_out" _returnvalue)))
  (Variables|Default|SetHologramActivated true))

(fn SetHologramPosition
  (params (Position :type Float%20%28single-precision%29))
  (bind _returnvalue (* Position 256.0))
  (bind _headertext (Variables|Default|GetHeaderText))
  (Transformation|SetWorldScale3D (Variables|Default|GetHologramm%20Area) (Math|Vector|MakeVector 0.005 (Variables|Default|GetHologramWidthScale) Position))
  (Transformation|SetRelativeLocation (Variables|Default|GetHologramm%20Area) (Math|Vector|MakeVector 0.0 (Variables|Default|GetHologramWidthScale) (* Position 128.0)) false)
  (Transformation|SetRelativeLocation (Variables|Default|GetTextRoot) (Math|Vector|MakeVector 0.0 (- (* (Variables|Default|GetHologramWidthScale) 128.0) 5.0) (- _returnvalue 3e+01)) false)
  (if (< (- _returnvalue 2e+01) (.X (Math|Vector|BreakVector (Class|TextRenderComponent|GetTextLocalSize _headertext))))
    (Rendering|SetVisibility (Variables|Default|GetHeaderText) false false)
    (else
      (Transformation|SetRelativeLocation _headertext (Math|Vector|MakeVector 0.0 0.0 (- _returnvalue 1e+01)) false))))

(fn PlayHologram
  (if (not (Variables|Default|GetHologramIsOpen))
    (if (< (Variables|Default|GetHologramCurrentPosition) (Variables|Default|GetHologramHeightScale))
      ;[0.036 1 0.1483] Open Hologram
      (if (>= (+ (Variables|Default|GetHologramCurrentPosition) (/ (Variables|Default|GetAnimationSpeed) 6e+01)) (Variables|Default|GetHologramHeightScale))
        (Variables|Default|SetHologramCurrentPosition (Variables|Default|GetHologramHeightScale))
        (else
          (Variables|Default|SetHologramCurrentPosition (+ (Variables|Default|GetHologramCurrentPosition) (/ (Variables|Default|GetAnimationSpeed) 6e+01)))))
      (CallFunction|SetHologramPosition (Variables|Default|GetHologramCurrentPosition))
      (else
        ;[1 0.9092 0.03979] Display Holorgram Massage
        (if (Variables|Default|GetTextIsPlaying)
          (CallFunction|CreateTextinLines (Variables|Default|GetShown%20Text))
          (else
            (CallFunction|SetTextVisibility true)
            (Variables|Default|SetTextIsPlaying true)))))
    (else
      ;[1 0.01836 0] Close Hologram
      (CallFunction|SetTextVisibility false)
      (if (> (Variables|Default|GetHologramCurrentPosition) 0.0)
        (if (< (- (Variables|Default|GetHologramCurrentPosition) (/ (Variables|Default|GetAnimationSpeed) 6e+01)) 0.0)
          (Variables|Default|SetHologramCurrentPosition 0.0)
          (else
            (Variables|Default|SetHologramCurrentPosition (- (Variables|Default|GetHologramCurrentPosition) (/ (Variables|Default|GetAnimationSpeed) 6e+01)))))
        (CallFunction|SetHologramPosition (Variables|Default|GetHologramCurrentPosition))
        (else
          (Variables|Default|SetHologramIsOpen false)
          (Variables|Default|SetHologramActivated false))))))

(fn CreateTextinLines
  (params (TextInput :type String))
  (bind _testtextline (Variables|Default|GetTestTextLine))
  (Variables|Default|SetThempText TextInput)
  (while (> (Utilities|String|Len (Variables|Default|GetThempText)) 0)
    ;[1 1 1] Use Test Line for checking the text length
    (Rendering|Components|TextRender|SetText _testtextline (Utilities|Text|ToText(String) (Variables|Default|GetThempText)))
    (if (> (.Y (Math|Vector|BreakVector (Class|TextRenderComponent|GetTextLocalSize _testtextline))) (* (Variables|Default|GetHologramWidthScale) 225.0))
      (CallFunction|BreakingTextAfterSpaces)
      (else
        (Utilities|Array|Add (Variables|Default|GetAllTextLines) (Variables|Default|GetThempText))
        (Variables|Default|SetThempText (Variables|Default|GetBreakingText))
        (Variables|Default|SetTextLeft "")
        (Variables|Default|SetBreakingText ""))))
  (switch Utilities|FlowControl|Switch|SwitchonE_HologramTextStyle (Variables|Default|GetTextStyle)
    (:NewEnumerator0
      (CallFunction|TextbyLines)
      (Variables|Default|SetHologramIsOpen true)
      (Variables|Default|SetHologramActivated false)
      (Variables|Default|SetTextIsPlaying false))))

(fn BreakingTextAfterSpaces
  ;[1 1 1] Split the text after a SPACE
  (Variables|Default|SetTextLeft (.LeftS (Utilities|String|Split (Variables|Default|GetThempText) " " "IgnoreCase" "FromEnd")))
  (if (> (Utilities|String|Len (Variables|Default|GetBreakingText)) 0)
    (Variables|Default|SetBreakingText (Utilities|String|Append (.RightS (Utilities|String|Split (Variables|Default|GetThempText) " " "IgnoreCase" "FromEnd")) " " (Variables|Default|GetBreakingText)))
    (else
      (Variables|Default|SetBreakingText (.RightS (Utilities|String|Split (Variables|Default|GetThempText) " " "IgnoreCase" "FromEnd")))))
  (Variables|Default|SetThempText (Variables|Default|GetTextLeft)))

(fn TextbyLines
  ;[1 1 1] Set the text in the lines
  (for (_array_element _array_index) (Variables|Default|GetAllTextLines)
    (switch int _array_index
      (:0
        (CallFunction|SetTexttoLine (Variables|Default|GetTextLine01) _array_element))
      (:1
        (CallFunction|SetTexttoLine (Variables|Default|GetTextLine02) _array_element))
      (:2
        (CallFunction|SetTexttoLine (Variables|Default|GetTextLine03) _array_element))
      (:3
        (CallFunction|SetTexttoLine (Variables|Default|GetTextLine04) _array_element))
      (:4
        (CallFunction|SetTexttoLine (Variables|Default|GetTextLine05) _array_element))
      (:5
        (CallFunction|SetTexttoLine (Variables|Default|GetTextLine06) _array_element))
      (:6
        (CallFunction|SetTexttoLine (Variables|Default|GetTextLine07) _array_element))
      (:7
        (CallFunction|SetTexttoLine (Variables|Default|GetTextLine08) _array_element))
      (:8
        (CallFunction|SetTexttoLine (Variables|Default|GetTextLine09) _array_element))
      (:9
        (CallFunction|SetTexttoLine (Variables|Default|GetTextLine10) _array_element)))))

(fn SetTexttoLine
  (params (TextLine :type Text%20Render%20Component%20Object%20Reference) (Text :type String))
  (Rendering|Components|TextRender|SetText TextLine (Utilities|Text|ToText(String) Text)))

(fn SetTextVisibility
  (params (Visible :type Boolean))
  (Rendering|SetVisibility (Variables|Default|GetTextLine01) Visible false))