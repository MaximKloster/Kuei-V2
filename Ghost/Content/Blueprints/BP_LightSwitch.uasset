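; Light switch actor that toggles a set of roof lamps whenever something overlaps its trigger.
; Each overlap flips IsOn, tilts the switch mesh to match, then casts each entry in the Lamps array to BP_RoofLamp and calls SetLight with the new state.
; The construction script sets the switch tilt from IsOn, but does not update the lamps.
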(event OnComponentBeginOverlap(Trigger)
  (params (OtherActor :type Actor%20Object%20Reference) (OtherComp :type Primitive%20Component%20Object%20Reference) (OtherBodyIndex :type Integer) (bFromSweep :type Boolean) (SweepResult :type Hit%20Result%20Structure%20%28by%20ref%29))
  (bind _switch (Variables|Default|GetSwitch))
  (if (Variables|Default|GetIsOn)
    (bind _output_get (Variables|Default|SetIsOn false))
    (Transformation|SetRelativeRotation _switch "-6.000000, 0, 0" false)
    (for _array_element (Variables|Default|Getlamps)
      (bind _asbp_roof_lamp (Utilities|Casting|CastToBP_RoofLamp _array_element))
      (Default|SetLight _asbp_roof_lamp _output_get))
    (else
      (bind _output_get_2 (Variables|Default|SetIsOn true))
      (Transformation|SetRelativeRotation _switch "6.000000, 0, 0" false)
      (for _array_element_2 (Variables|Default|Getlamps)
        (bind _asbp_roof_lamp_2 (Utilities|Casting|CastToBP_RoofLamp _array_element_2))
        (Default|SetLight _asbp_roof_lamp_2 _output_get_2)))))

(fn ConstructionScript
  (bind _switch (Variables|Default|GetSwitch))
  (if (Variables|Default|GetIsOn)
    (Transformation|SetRelativeRotation _switch "6.000000, 0, 0" false)
    (else
      (Transformation|SetRelativeRotation _switch "-6.000000, 0, 0" false))))