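; Scaled hero Blueprint that resizes itself uniformly to follow the PlayerSize value of a referenced player scaler.
; Every Tick it divides that size by a fixed baseline and applies the result as the Root's world scale on all axes.
; The construction script computes the same Scaler value but does not apply it, so resizing happens only on Tick.
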(event EventBeginPlay)

(event Collision|EventActorBeginOverlap
  (params (OtherActor :type Actor%20Object%20Reference)))

(event EventTick
  (params (DeltaSeconds :type Float%20%28single-precision%29))
  (Variables|Default|SetScaler (/ (Variables|/Game/Blueprints/BP_Player_Scaler.BP_Player_Scaler_C|GetPlayerSize (Variables|Default|GetPlayerScalerRef)) 2e+02))
  (Transformation|SetWorldScale3D (Variables|Default|Getroot) (Math|Vector|MakeVector (Variables|Default|GetScaler) (Variables|Default|GetScaler) (Variables|Default|GetScaler))))

(fn ConstructionScript
  (Variables|Default|SetScaler (/ (Variables|/Game/Blueprints/BP_Player_Scaler.BP_Player_Scaler_C|GetPlayerSize (Variables|Default|GetPlayerScalerRef)) 2e+02)))