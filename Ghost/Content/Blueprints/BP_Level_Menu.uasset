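; BP_Level_Menu is a level-select menu actor that saves the player's body measurements and opens a named level when touched.
; ActivateMenu stores player size and arm length, shows its text and targets half the player's size as height.
; Tick moves it up in fixed, frame-dependent steps, enabling interaction at the top.
; Trigger overlap by BP_Initialisation_Charakter then writes a fresh PlayerSaves slot and loads the level.
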(event OnComponentBeginOverlap(Trigger)
  (params (OtherActor :type Actor%20Object%20Reference) (OtherComp :type Primitive%20Component%20Object%20Reference) (OtherBodyIndex :type Integer) (bFromSweep :type Boolean) (SweepResult :type Hit%20Result%20Structure%20%28by%20ref%29))
  ;[1 0.9775 0] If the button is activated save player stats and load the level
  (if (Variables|Default|GetInteractable)
    (Utilities|Casting|CastToBP_Initialisation_Charakter OtherActor)
    (CallFunction|SavePlayerStats)
    (Game|OpenLevel(byName) (Variables|Default|GetLevelName))))

(event EventTick
  (params (DeltaSeconds :type Float%20%28single-precision%29))
  (bind _root (Variables|Default|Getroot))
  (bind _root_2 (Variables|Default|Getroot))
  (bind _returnvalue (Transformation|GetWorldLocation _root_2))
  (bind _returnvalue_2 (Transformation|GetWorldLocation _root))
  (bind (_x _y _z) (Math|Vector|BreakVector _returnvalue))
  (bind (_x_2 _y_2 _z_2) (Math|Vector|BreakVector _returnvalue_2))
  ;[1 0 0.9038] Menu activation animation
  (if (Variables|Default|GetMenuActivated)
    (if (<= _z (Variables|Default|GetMenuHight))
      (Transformation|SetWorldLocation _root_2 (Math|Vector|MakeVector _x _y (+ _z 0.25)) false)
      (else
        (Variables|Default|SetInteractable true)))
    (else
      (Variables|Default|SetInteractable false)
      (if (> _z_2 2e+01)
        (Transformation|SetWorldLocation _root (Math|Vector|MakeVector _x_2 _y_2 (- _z_2 0.25)) false)))))

(fn ConstructionScript
  (bind _root (Variables|Default|Getroot))
  (bind _returnvalue (Transformation|GetWorldLocation _root))
  (bind (_x _y) (Math|Vector|BreakVector _returnvalue))
  (Transformation|SetWorldLocation _root (Math|Vector|MakeVector _x _y (Variables|Default|GetStartHigh)) false))

(fn ActivateMenu
  (params (PlayerSize :type Float%20%28single-precision%29 :default 0.0) (ArmLength :type Float%20%28single-precision%29))
  (Variables|Default|SetPlayerSize PlayerSize)
  (Variables|Default|SetMenuHight (/ PlayerSize 2.0))
  (Variables|Default|SetArmLength ArmLength)
  (Variables|Default|SetMenuActivated true)
  (Rendering|SetVisibility (Variables|Default|GetTextRender) true false))

(fn SavePlayerStats
  (bind _returnvalue (SaveGame|CreateSaveGameObject "/Game/Blueprints/PlayerSaves.PlayerSaves_C"))
  (bind _asplayer_saves (Utilities|Casting|CastToPlayerSaves _returnvalue))
  (bind _output_get (Variables|Default|SetPlayerSavesInstance _asplayer_saves))
  (Variables|/Game/Blueprints/PlayerSaves.PlayerSaves_C|SetPlayerSize _output_get (Variables|Default|GetPlayerSize))
  (Variables|/Game/Blueprints/PlayerSaves.PlayerSaves_C|SetArmLength _output_get (Variables|Default|GetArmLength))
  (SaveGame|SaveGametoSlot _output_get (Variables|/Game/Blueprints/PlayerSaves.PlayerSaves_C|GetSaveSlotName _output_get) (Variables|/Game/Blueprints/PlayerSaves.PlayerSaves_C|GetUser%20Index _output_get)))