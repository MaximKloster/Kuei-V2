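; Physics object that player hands can interact with, using Kinect character hand states and drag-character hand collisions.
; A trigger overlap checks hand tag and state, then disables mesh physics and collision when interaction is possible.
; Tagged hand overlaps on the mesh drive Tick, which offsets its location and toggles gravity.
; Grab-and-throw logic, with socket attachment and force from recent hand positions, is present but disconnected.
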(event OnComponentEndOverlap(Trigger)
  (params (OtherActor :type Actor%20Object%20Reference) (OtherComp :type Primitive%20Component%20Object%20Reference) (OtherBodyIndex :type Integer))
  ;[1 1 1] A Player Hand is not more in the Interaction Range
  (CallFunction|CheckHand OtherActor OtherComp)
  (if (not (Variables|Default|GetIsInRightHand))
    (if (not (Variables|Default|GetIsInLeftHand))
      (if (== (Variables|Default|GetHand) 1)
        _))))

(event OnComponentBeginOverlap(Mesh)
  (params (OtherActor :type Actor%20Object%20Reference) (OtherComp :type Primitive%20Component%20Object%20Reference) (OtherBodyIndex :type Integer) (bFromSweep :type Boolean) (SweepResult :type Hit%20Result%20Structure%20%28by%20ref%29))
  (bind _returnvalue (Transformation|GetWorldLocation OtherComp))
  ;[1 1 1] Check and set active hand changing for this object
  (bind _asbp_optimized_drag_charakter (Utilities|Casting|CastToBP_Optimized_Drag_Charakter OtherActor))
  (Variables|Default|SetCharakter _asbp_optimized_drag_charakter)
  (if (Components|ComponentHasTag OtherComp "RightHandCollision")
    (Variables|Default|SetMovingByRightHand true)
    (Variables|Default|SetPositionChangeByRightHand _returnvalue)
    (elif (Components|ComponentHasTag OtherComp "LeftHandCollision")
      (Variables|Default|SetMovingByLeftHand true)
      (Variables|Default|SetPositionChangeByLeftHand _returnvalue))))

(event OnComponentBeginOverlap(Trigger)
  (params (OtherActor :type Actor%20Object%20Reference) (OtherComp :type Primitive%20Component%20Object%20Reference) (OtherBodyIndex :type Integer) (bFromSweep :type Boolean) (SweepResult :type Hit%20Result%20Structure%20%28by%20ref%29))
  (bind _mesh (Variables|Default|GetMesh))
  ;[1 1 1] A Player Hand is in Interaction Range of the Object, deactivate Collision for possible interaction
  (CallFunction|CheckHand OtherActor OtherComp)
  (if (== (Variables|Default|GetHand) 1)
    (if (Variables|Default|GetIsInInteractionRight)
      (Physics|SetSimulatePhysics _mesh false :!label _label)
      (Collision|SetCollisionEnabled _mesh "NoCollision"))
    (elif (Variables|Default|GetIsInInteractionLeft)
      (goto _label))))

(event OnComponentEndOverlap(Mesh)
  (params (OtherActor :type Actor%20Object%20Reference) (OtherComp :type Primitive%20Component%20Object%20Reference) (OtherBodyIndex :type Integer))
  ;[1 1 1] Remove active hand if its not more overlaped
  (Utilities|Casting|CastToBP_Optimized_Drag_Charakter OtherActor)
  (if (Components|ComponentHasTag OtherComp "RightHandCollision")
    (Variables|Default|SetMovingByRightHand false)
    (elif (Components|ComponentHasTag OtherComp "LeftHandCollision")
      (Variables|Default|SetMovingByLeftHand false))))

(event EventTick
  (params (DeltaSeconds :type Float%20%28single-precision%29))
  (bind _charakter (Variables|Default|GetCharakter))
  (bind _positionchangebyrighthand (Variables|Default|GetPositionChangeByRightHand))
  (bind _mesh (Variables|Default|GetMesh))
  (bind _positionchangebylefthand (Variables|Default|GetPositionChangeByLeftHand))
  (bind _returnvalue (Transformation|GetWorldLocation _mesh))
  (bind _returnvalue_2 (Transformation|GetWorldLocation _charakter))
  (bind _returnvalue_3 (- _returnvalue_2 _positionchangebylefthand))
  (bind _returnvalue_4 (- _returnvalue_2 _positionchangebyrighthand))
  ;[1 1 1] Position changes by righ hand in action
  (if (Variables|Default|GetMovingByRightHand)
    (Physics|SetEnableGravity _mesh (< (.Z (Math|Vector|BreakVector _returnvalue_4)) 0.0))
    (Transformation|SetWorldLocation _mesh (+ _returnvalue_4 _returnvalue) false)
    (else
      ;[1 1 1] Position changes by left hand in action
      (if (Variables|Default|GetMovingByLeftHand)
        (Physics|SetEnableGravity _mesh (< (.Z (Math|Vector|BreakVector _returnvalue_3)) 0.0))
        (Transformation|SetWorldLocation _mesh (+ _returnvalue _returnvalue_3) false)
        (else
          (Physics|SetEnableGravity _mesh true))))))

(fn ConstructionScript)

(fn CheckHand
  (params (Actor :type Actor%20Object%20Reference) (ActorComponent :type Actor%20Component%20Object%20Reference))
  (bind _asbp_kinect_character (Utilities|Casting|CastToBP_Kinect_Character Actor))
  (Variables|Default|SetPlayer _asbp_kinect_character)
  (for _array_element (Variables|/Script/Engine.ActorComponent|GetComponentTags ActorComponent)
    (if (Utilities|Name|Equal(Name) _array_element (Variables|/Game/Blueprints/BP_Kinect_Character.BP_Kinect_Character_C|GetRightHandCollisionTag _asbp_kinect_character))
      (Variables|Default|SetHand "Right")
      (if (== (Variables|/Game/Blueprints/BP_Kinect_Character.BP_Kinect_Character_C|GetRightHandState _asbp_kinect_character) 2)
        (Variables|Default|SetIsInInteractionRight true)
        (else
          (Variables|Default|SetIsInInteractionRight false)))
      (elif (Utilities|Name|Equal(Name) _array_element (Variables|/Game/Blueprints/BP_Kinect_Character.BP_Kinect_Character_C|GetLeftHandCollisionTag _asbp_kinect_character))
        (Variables|Default|SetHand "Left")
        (if (== (Variables|/Game/Blueprints/BP_Kinect_Character.BP_Kinect_Character_C|GetLeftHandState _asbp_kinect_character) 2)
          (Variables|Default|SetIsInInteractionLeft true)
          (else
            (Variables|Default|SetIsInInteractionLeft false)))))))

(fn ThrowObject
  (params (Hand :type EHands%20Enum :default "Left") (Player :type BP%20Kinect%20Character%20Object%20Reference) (ForceFactor :type Float%20%28single-precision%29 :default 0.0))
  (bind _kinectmesh (Variables|/Game/Blueprints/BP_Kinect_Character.BP_Kinect_Character_C|GetKinectMesh Player))
  (bind _mesh (Variables|Default|GetMesh))
  (bind _holdinghandpositionsright (Variables|Default|GetHoldingHandPositionsRight))
  (bind _holdinghandpositionsleft (Variables|Default|GetHoldingHandPositionsLeft))
  (bind _mesh_2 (Variables|Default|GetMesh))
  (Class|SceneComponent|DetachfromParent _mesh false true)
  (if (== Hand 1)
    ;[1 1 1] Throw Object from Right Hand
    (Variables|Default|SetIsInRightHand false)
    (bind (_outposition _outrotation) (Class|SkinnedMeshComponent|TransformfromBoneSpace _kinectmesh "middle_01_r" "0, 0, 0" "0, 0, 0"))
    (Transformation|SetWorldLocationAndRotation _mesh _outposition _outrotation false)
    (Collision|SetCollisionEnabled _mesh "QueryAndPhysics")
    (Physics|SetSimulatePhysics _mesh true)
    (CallFunction|CalculateForce (Utilities|Array|Get(acopy) _holdinghandpositionsright) (Utilities|Array|Get(acopy) _holdinghandpositionsright (- (Utilities|Array|Length _holdinghandpositionsright) 1)) ForceFactor)
    (Physics|AddForce _mesh (Variables|Default|GetThrowingForce) "None" false)
    (else
      ;[1 1 1] Throw Object from Left Hand
      (Variables|Default|SetIsInRightHand false)
      (bind (_outposition_2 _outrotation_2) (Class|SkinnedMeshComponent|TransformfromBoneSpace _kinectmesh "middle_01_l" "0, 0, 0" "0, 0, 0"))
      (Transformation|SetWorldLocationAndRotation _mesh_2 _outposition_2 _outrotation_2 false)
      (Collision|SetCollisionEnabled _mesh_2 "QueryAndPhysics")
      (Physics|SetSimulatePhysics _mesh_2 true)
      (CallFunction|CalculateForce (Utilities|Array|Get(acopy) _holdinghandpositionsleft) (Utilities|Array|Get(acopy) _holdinghandpositionsleft (- (Utilities|Array|Length _holdinghandpositionsleft) 1)) ForceFactor)
      (Physics|AddForce _mesh_2 (Variables|Default|GetThrowingForce) "None" false))))

(fn CalculateForce
  (params (FirstPosition :type Vector :default "0, 0, 0") (LastPosition :type Vector :default "0, 0, 0") (Factor :type Float%20%28single-precision%29 :default 0.0))
  (bind (_x _y _z) (Math|Vector|BreakVector FirstPosition))
  (bind (_x_2 _y_2 _z_2) (Math|Vector|BreakVector LastPosition))
  (bind _returnvalue (- _x_2 _x))
  (bind _returnvalue_2 (- _y_2 _y))
  (bind _returnvalue_3 (- _z_2 _z))
  (bind _returnvalue_4 (* _returnvalue Factor))
  (bind _returnvalue_5 (* _returnvalue_2 Factor))
  (bind _returnvalue_6 (* _returnvalue_3 Factor))
  (bind _returnvalue_7 (Math|Vector|MakeVector _returnvalue_4 _returnvalue_5 _returnvalue_6))
  (Variables|Default|SetThrowingForce _returnvalue_7)
  (Development|PrintText (Utilities|Text|ToText(Float) (Math|Vector|VectorLength _returnvalue_7) "HalfToEven")))

(fn ObjectWayinHand
  (params (Hand :type EHands%20Enum :default "Left") (Player :type BP%20Kinect%20Character%20Object%20Reference))
  (bind _kinectmesh (Variables|/Game/Blueprints/BP_Kinect_Character.BP_Kinect_Character_C|GetKinectMesh Player))
  (if (== Hand 1)
    ;[1 1 1] Set Right Hand Positions Array
    (bind _outposition (Class|SkinnedMeshComponent|TransformfromBoneSpace _kinectmesh "middle_01_r" "0, 0, 0" "0, 0, 0"))
    (if (>= (Utilities|Array|Length (Variables|Default|GetHoldingHandPositionsRight)) 6)
      (bind _output_get (Variables|Default|SetThemporaryPositionsArray (Utilities|Array|MakeArray (Utilities|Array|Get(acopy) (Variables|Default|GetHoldingHandPositionsRight) 1) (Utilities|Array|Get(acopy) (Variables|Default|GetHoldingHandPositionsRight) 2) (Utilities|Array|Get(acopy) (Variables|Default|GetHoldingHandPositionsRight) 3) (Utilities|Array|Get(acopy) (Variables|Default|GetHoldingHandPositionsRight) 4) (Utilities|Array|Get(acopy) (Variables|Default|GetHoldingHandPositionsRight) 5) _outposition)))
      (Variables|Default|SetHoldingHandPositionsRight _output_get)
      (else
        (Utilities|Array|Add (Variables|Default|GetHoldingHandPositionsRight) _outposition)))
    (else
      ;[1 1 1] Set Left Hand Positions Array
      (bind _outposition_2 (Class|SkinnedMeshComponent|TransformfromBoneSpace _kinectmesh "None" "0, 0, 0" "0, 0, 0"))
      (if (>= (Utilities|Array|Length (Variables|Default|GetHoldingHandPositionsLeft)) 6)
        (bind _output_get_2 (Variables|Default|SetThemporaryPositionsArray (Utilities|Array|MakeArray (Utilities|Array|Get(acopy) (Variables|Default|GetHoldingHandPositionsLeft) 1) (Utilities|Array|Get(acopy) (Variables|Default|GetHoldingHandPositionsLeft) 2) (Utilities|Array|Get(acopy) (Variables|Default|GetHoldingHandPositionsLeft) 3) (Utilities|Array|Get(acopy) (Variables|Default|GetHoldingHandPositionsLeft) 4) (Utilities|Array|Get(acopy) (Variables|Default|GetHoldingHandPositionsLeft) 5) _outposition_2)))
        (Variables|Default|SetHoldingHandPositionsLeft _output_get_2)
        (else
          (Utilities|Array|Add (Variables|Default|GetHoldingHandPositionsLeft) _outposition_2)))))
  (return Player))