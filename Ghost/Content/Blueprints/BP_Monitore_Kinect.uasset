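; BP_Monitore_Kinect is an in-world monitor that shows a live Kinect camera feed of a configurable camera type.
; Overlapping its Box toggles IsOn, and BeginPlay applies the initial state.
; When on, it lights the PointLight, puts the camera frame texture on a dynamic Display material and enables frame updating.
; When off, it hides the light and restores the default display material, without disabling frame updating.
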(event OnComponentBeginOverlap(Box)
  (params (OtherActor :type Actor%20Object%20Reference) (OtherComp :type Primitive%20Component%20Object%20Reference) (OtherBodyIndex :type Integer) (bFromSweep :type Boolean) (SweepResult :type Hit%20Result%20Structure%20%28by%20ref%29))
  (if (Variables|Default|GetIsOn)
    ;[1 1 1] The monitore is off
    (bind _output_get (Variables|Default|SetIsOn false))
    (Rendering|SetVisibility (Variables|Components|GetPointLight) _output_get false)
    (Rendering|Material|SetMaterial (Variables|Components|GetDisplay) 0 "/Game/Materials/M_Monitore_Display.M_Monitore_Display")
    (else
      ;[1 1 1] The monitore is on and show the kinect type, that is switched
      (bind _output_get_2 (Variables|Default|SetIsOn true))
      (Rendering|SetVisibility (Variables|Components|GetPointLight) _output_get_2 false)
      (bind _returnvalue (Class|KinectInterfaceComponent|GetCameraFrame (Variables|Components|GetKinectInterface) (Variables|Default|GetKinectCameraType)))
      (bind _returnvalue_2 (Rendering|Material|CreateDynamicMaterialInstance (Variables|Components|GetDisplay) 0 "/Game/Materials/M_Dynamic_Material.M_Dynamic_Material" :!class /Script/Engine.PrimitiveComponent))
      (Rendering|Material|SetTextureParameterValue _returnvalue_2 "Texture" _returnvalue)
      (Class|KinectInterfaceComponent|SetCameraFrameIsUpdating (Variables|Components|GetKinectInterface) (Variables|Default|GetKinectCameraType) true))))

(event EventBeginPlay
  (if (not (Variables|Default|GetIsOn))
    ;[1 1 1] The monitore is off
    (Rendering|SetVisibility (Variables|Components|GetPointLight) (stale OnComponentBeginOverlap(Box) _output_get) false)
    (Rendering|Material|SetMaterial (Variables|Components|GetDisplay) 0 "/Game/Materials/M_Monitore_Display.M_Monitore_Display")
    (else
      ;[1 1 1] The monitore is on and show the kinect type, that is switched
      (Rendering|SetVisibility (Variables|Components|GetPointLight) (stale OnComponentBeginOverlap(Box) _output_get_2) false)
      (bind _returnvalue (Class|KinectInterfaceComponent|GetCameraFrame (Variables|Components|GetKinectInterface) (Variables|Default|GetKinectCameraType)))
      (bind _returnvalue_2 (Rendering|Material|CreateDynamicMaterialInstance (Variables|Components|GetDisplay) 0 "/Game/Materials/M_Dynamic_Material.M_Dynamic_Material" :!class /Script/Engine.PrimitiveComponent))
      (Rendering|Material|SetTextureParameterValue _returnvalue_2 "Texture" _returnvalue)
      (Class|KinectInterfaceComponent|SetCameraFrameIsUpdating (Variables|Components|GetKinectInterface) (Variables|Default|GetKinectCameraType) true))))

(fn ConstructionScript)